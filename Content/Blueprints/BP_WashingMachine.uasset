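; BP_WashingMachine is a washing machine actor that exposes events for a wash cycle and for upgrades.
; StartWashCycle and EndWashCycle snap WashDoor to its ClosePos or OpenPos yaw, with no animation or cycle timing in this graph.
; UpgradeEvent switches on UpgradeState to swap the MachineMesh static mesh for the Medium and Large tiers, using what look like placeholder shapes (a cone and a bush).
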(event `self.K2_StartWashCycle`
  ;[1 1 1] Gameplay Cue events
  (`SceneComponent.K2_SetRelativeRotation` (`self.WashDoor`) (`KismetMathLibrary.MakeRotator` 0.0 0.0 (`self.ClosePos`)) false false))

(event `self.K2_EndWashCycle`
  ;[1 1 1] Gameplay Cue events
  (`SceneComponent.K2_SetRelativeRotation` (`self.WashDoor`) (`KismetMathLibrary.MakeRotator` 0.0 0.0 (`self.OpenPos`)) false false))

(event `self.K2_UpgradeEvent`
  ;[1 1 1] Gameplay Cue events
  (switch `EMachineUpgrade` (`self.UpgradeState`)
    (:`MEDIUM`
      (`StaticMeshComponent.SetStaticMesh` (`self.MachineMesh`) "/Game/StarterContent/Shapes/Shape_Cone.Shape_Cone"))
    (:`LARGE`
      (`StaticMeshComponent.SetStaticMesh` (`self.MachineMesh`) "/Game/AshStuff/AshsAssets/BushWorking/bush.bush"))))

(fn `UserConstructionScript`)