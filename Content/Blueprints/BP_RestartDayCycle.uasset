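; A trigger actor that restarts the shop's day cycle in the laundry game when a pawn overlaps its DayRestart component.
; BeginPlay caches the BP_ShopDayCycle game instance and the level's LaundryManager, and the overlap acts only while GameState is 1.
; StartNewDay destroys leftover bags, reinitializes the day cycle, then restarts the laundry spawn timer.
; Fade-in and player repositioning are still marked TODO.
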(event `self.ReceiveBeginPlay`
  (bind _asbp_shop_day_cycle (cast `/Game/DayCycleGameInstance/BP_ShopDayCycle` (`GameplayStatics.GetGameInstance`)))
  (set `self.GameInstanceRef` _asbp_shop_day_cycle)
  (bind _returnvalue (`GameplayStatics.GetActorOfClass` "/Script/FrontierJam.LaundryManager"))
  (set `self.LaundryManagerRef` _returnvalue))

(event `self.DayRestart.OnComponentBeginOverlap`
  (params (OverlappedComponent :type "PrimitiveComponent Object Reference") (OtherActor :type "Actor Object Reference") (OtherComp :type "PrimitiveComponent Object Reference") (OtherBodyIndex :type Integer) (bFromSweep :type Boolean) (SweepResult :type "HitResult Structure (by ref)"))
  ;[1 0 0.1048] Restarts the day cycle
  ; TODO -- Fade In and move player to correct position
  (if (== (`ShopDayCycle.GameState` (`self.GameInstanceRef`)) 1)
    (cast `Pawn` OtherActor)
    (`KismetSystemLibrary.PrintString` "Restart Day")
    (`self.StartNewDay`)))

(fn `StartNewDay`
  (`KismetSystemLibrary.PrintString` "All bags gone")
  (`LaundryManager.DestroyAllLeftoverBags` (`self.LaundryManagerRef`))
  (`ShopDayCycle.InitializeDayCycle` (`self.GameInstanceRef`))
  (`LaundryManager.InitializeLaundrySpawnTimer` (`self.LaundryManagerRef`)))

(fn `UserConstructionScript`)